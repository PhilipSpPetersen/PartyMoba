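; Camera actor that becomes the player's view target on BeginPlay and follows player character 0 within map bounds.
; A Tick gate, toggled by StartCamFollow and StopCamFollow, runs separate X and Y checks against MapCenter plus min/max offsets.
; While the player is inside an axis's bounds, VInterpTo moves the camera on that axis and also toward the player's Z.
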(event `self.ReceiveBeginPlay`
  ;[1 1 1] Start/Stop Cam Follow
  (`PlayerController.SetViewTargetWithBlend` (`GameplayStatics.GetPlayerController` 0) self 0.0 "VTBlend_Linear" 0.0 false)
  (`self.StartCamFollow`))

(event `self.ReceiveTick`
  (params (DeltaSeconds :type "Float (single-precision)"))
  ;[1 1 1] Start/Stop Cam Follow Function
  (`/Engine/EditorBlueprintResources/StandardMacros.Gate` true :!label _label
    (:`Exit`
      (`self.CheckPlayerX`)
      (`self.CheckPlayerY`))))

(event `StartCamFollow`
  ;[1 1 1] Start/Stop Cam Follow Function
  (goto _label :!via `Open`))

(event `StopCamFollow`
  ;[1 1 1] Start/Stop Cam Follow Function
  (goto _label :!via `Close`))

(event `CheckPlayerX`
  (bind _returnvalue_x (`KismetMathLibrary.BreakVector` (`self.K2_GetActorLocation` (`GameplayStatics.GetPlayerCharacter` 0))))
  (bind _returnvalue_x_2 (`KismetMathLibrary.BreakVector` (`self.K2_GetActorLocation` (`GameplayStatics.GetPlayerCharacter` 0))))
  ;[1 1 1] Move Camera X
  (if (and (> _returnvalue_x (+ (`self.MapCenter`) (`self.MinX`))) (< _returnvalue_x_2 (+ (`self.MapCenter`) (`self.MaxX`))))
    (`self.MoveCameraX`)))

(event `MoveCameraX`
  (bind (_returnvalue_x _returnvalue_y) (`KismetMathLibrary.BreakVector` (`self.K2_GetActorLocation`)))
  (bind (_returnvalue_x_2 _returnvalue_y_2 _returnvalue_z) (`KismetMathLibrary.BreakVector` (`self.K2_GetActorLocation` (`GameplayStatics.GetPlayerCharacter` 0))))
  ;[1 1 1] Move Camera X Function
  (`self.K2_SetActorLocation` (`KismetMathLibrary.VInterpTo` (`self.K2_GetActorLocation`) (`KismetMathLibrary.MakeVector` _returnvalue_x_2 _returnvalue_y _returnvalue_z) (`GameplayStatics.GetWorldDeltaSeconds`))))

(event `CheckPlayerY`
  (bind (_returnvalue_x _returnvalue_y) (`KismetMathLibrary.BreakVector` (`self.K2_GetActorLocation` (`GameplayStatics.GetPlayerCharacter` 0))))
  (bind (_returnvalue_x_2 _returnvalue_y_2) (`KismetMathLibrary.BreakVector` (`self.K2_GetActorLocation` (`GameplayStatics.GetPlayerCharacter` 0))))
  ;[1 1 1] Move Camera Y
  (if (and (> _returnvalue_y (+ (`self.MapCenter`) (`self.MinY`))) (< _returnvalue_y_2 (+ (`self.MapCenter`) (`self.MaxY`))))
    (`self.MoveCameraY`)))

(event `MoveCameraY`
  (bind _returnvalue_x (`KismetMathLibrary.BreakVector` (`self.K2_GetActorLocation`)))
  (bind (_returnvalue_x_2 _returnvalue_y _returnvalue_z) (`KismetMathLibrary.BreakVector` (`self.K2_GetActorLocation` (`GameplayStatics.GetPlayerCharacter` 0))))
  ;[1 1 1] Move Camera Y Function
  (`self.K2_SetActorLocation` (`KismetMathLibrary.VInterpTo` (`self.K2_GetActorLocation`) (`KismetMathLibrary.MakeVector` _returnvalue_x _returnvalue_y _returnvalue_z) (`GameplayStatics.GetWorldDeltaSeconds`))))

(fn `UserConstructionScript`)