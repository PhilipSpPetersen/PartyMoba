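; BP_Rock is a pickup actor that adds rock ammo to the warrior player.
; On BeginPlay it enables input from the first player controller so it can receive the Pickup action directly.
; Overlap events on PickupCol cache the warrior and open or close a Gate, so a press only counts while in range.
; A successful pickup increments the warrior's RockAmmo and destroys the rock.
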(event `self.ReceiveBeginPlay`
  ;[1 1 1] Enable Pickup
  (`self.EnableInput` (`GameplayStatics.GetPlayerController` 0)))

(event `InputAction|Pickup` :consume false
  (params (Key :type "Key Structure"))
  ;[1 1 1] Pickup
  (:`Pressed`
    (`/Engine/EditorBlueprintResources/StandardMacros.Gate` true :!label _label
      (:`Exit`
        (bind _result (`/Engine/EditorBlueprintResources/StandardMacros.IncrementInt` (`/Game/_Main/BP_Player_Warrior.RockAmmo` (stale `self.PickupCol.OnComponentBeginOverlap` _asbp_player_warrior)))
          (:`  `
            (set `/Game/_Main/BP_Player_Warrior.RockAmmo` _result (stale `self.PickupCol.OnComponentBeginOverlap` _asbp_player_warrior))
            (`self.K2_DestroyActor`)))))))

(event `self.PickupCol.OnComponentBeginOverlap`
  (params (OverlappedComponent :type "PrimitiveComponent Object Reference") (OtherActor :type "Actor Object Reference") (OtherComp :type "PrimitiveComponent Object Reference") (OtherBodyIndex :type Integer) (bFromSweep :type Boolean) (SweepResult :type "HitResult Structure (by ref)"))
  ;[1 1 1] Pickup
  (bind _asbp_player_warrior (cast `/Game/_Main/BP_Player_Warrior` OtherActor))
  (goto _label :!via `Open`))

(event `self.PickupCol.OnComponentEndOverlap`
  (params (OverlappedComponent :type "PrimitiveComponent Object Reference") (OtherActor :type "Actor Object Reference") (OtherComp :type "PrimitiveComponent Object Reference") (OtherBodyIndex :type Integer))
  ;[1 1 1] Pickup
  (cast `/Game/_Main/BP_Player_Warrior` OtherActor)
  (goto _label :!via `Close`))

(fn `UserConstructionScript`)