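; BP_Hammer is a hammer weapon that the warrior player can pick up and equip.
; Its PickUpWeapon event detaches any weapon the player already holds and moves it to the hammer's location and rotation, swapping the two.
; It then sets itself as the player's EquipWeapon and attaches to the character mesh at the weapon_equipped socket.
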(event `/Game/_Main/InteractWithWeapon.Pick Up Weapon`
  (bind _defaultsceneroot (`self.DefaultSceneRoot`))
  (bind _asbp_player_warrior (cast `/Game/_Main/BP_Player_Warrior` (`GameplayStatics.GetPlayerCharacter` 0) :!pure true))
  (bind _equipweapon (`/Game/_Main/BP_Player_Warrior.EquipWeapon` (cast `/Game/_Main/BP_Player_Warrior` (`GameplayStatics.GetPlayerCharacter` 0) :!pure true)))
  ;[1 1 1] Pick Up Weapon
  (`/Engine/EditorBlueprintResources/StandardMacros.IsValid` _equipweapon
    (:`Is Valid`
      (`self.K2_DetachFromActor` _equipweapon "KeepRelative" "KeepRelative" "KeepRelative")
      (`self.K2_SetActorLocationAndRotation` _equipweapon (`SceneComponent.K2_GetComponentLocation` _defaultsceneroot) (`SceneComponent.K2_GetComponentRotation` _defaultsceneroot) false false))
    (:`Is Not Valid`
      _))
  (set `/Game/_Main/BP_Player_Warrior.EquipWeapon` self _asbp_player_warrior)
  (`self.K2_AttachToComponent` (`Character.Mesh` _asbp_player_warrior) "weapon_equipped" "SnapToTarget" "SnapToTarget" "KeepRelative"))

(fn `UserConstructionScript`)